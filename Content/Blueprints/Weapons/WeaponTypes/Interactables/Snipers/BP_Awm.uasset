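; BP_Awm is the AWM sniper interactable weapon, extending its parent's information panel setup with a scope panel.
; It appends ScopeInfoPanel to the inherited InfoPanels array.
; SetPanelRefs runs the parent logic, then links the ScopeHotspot button widget to the scope's weapon information widget.
; The event graph holds only disabled stubs, and the construction script just calls the parent.
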(fn `CreateInfoPanelsArray`
  (`parent.CreateInfoPanelsArray`)
  (`KismetArrayLibrary.Array_Add` (`self.InfoPanels`) (`self.ScopeInfoPanel`)))

(fn `SetPanelRefs`
  (`parent.SetPanelRefs`)
  (bind _aswbp_info_panel_button (cast `/Game/Blueprints/UI/3DWeaponCatalog/WBP_InfoPanelButton` (`WidgetComponent.GetUserWidgetObject` (`self.ScopeHotspot`))))
  (bind _aswbp_weapon_information_panel (cast `/Game/Blueprints/UI/3DWeaponCatalog/WBP_WeaponInformationPanel` (`WidgetComponent.GetUserWidgetObject` (`self.ScopeInfoPanel`))))
  (set `/Game/Blueprints/UI/3DWeaponCatalog/WBP_InfoPanelButton.InfoPanelRef` _aswbp_weapon_information_panel _aswbp_info_panel_button))

(fn `UserConstructionScript`
  (`parent.UserConstructionScript`))