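; Base Blueprint for interactable weapons that present weapon, ammo and magazine information through hotspot widgets.
; On BeginPlay it links each hotspot button to its info panel, then looks up its WeaponName row in the game instance's InteractableWeaponsData table.
; The row's HotSpots entries fill the panels' heading, description and image by array index.
; Equip, unequip and attachment-map update functions are empty stubs, apparently for child weapons to override.
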(event `self.ReceiveBeginPlay`
  (`parent.ReceiveBeginPlay`)
  (`self.SetPanelRefs`)
  (`self.CreateInfoPanelsArray`)
  (bind _asbp_uigame_instance (cast `/Game/Blueprints/BP_UIGameInstance` (`GameplayStatics.GetGameInstance`)))
  (bind _output_get (set `self.GameInstRef` _asbp_uigame_instance))
  (bind _returnvalue (`|GetDataTableRow` (`/Game/Blueprints/BP_UIGameInstance.InteractableWeaponsData` _output_get) (`self.WeaponName`))
    (:`then`
      (`self.SetData` _returnvalue)
      (`self.UpdateAttachmentMap`))))

(fn `CreateInfoPanelsArray`
  (`KismetArrayLibrary.Array_Add` (`self.InfoPanels`) (`self.WeaponInfoPanel`))
  (`KismetArrayLibrary.Array_Add` (`self.InfoPanels`) (`self.AmmoInfoPanel`))
  (`KismetArrayLibrary.Array_Add` (`self.InfoPanels`) (`self.MagazineInfoPanel`)))

(fn `EquipAttachment`
  (params (AttachmentType :type "/Game/Blueprints/Weapons/EAttachmentType Enum" :default "NewEnumerator0")))

(fn `SetData`
  (params (WeaponData :type "/Game/Blueprints/Weapons/InteractableWeaponData/FInteractableWeaponTableRowBase Structure"))
  (set `self.WeaponData` WeaponData)
  (`self.SetHotspots`))

(fn `SetHotspots`
  (bind (_weapondata_weaponname _weapondata_weaponimage _weapondata_hotspots) (break `/Game/Blueprints/Weapons/InteractableWeaponData/FInteractableWeaponTableRowBase` (`self.WeaponData`)))
  (for (_array_element _array_index) _weapondata_hotspots
    (bind _output (`|GetArrayItem` (`self.InfoPanels`) _array_index))
    (`/Engine/EditorBlueprintResources/StandardMacros.IsValid` _output
      (:`Is Valid`
        (bind _aswbp_weapon_information_panel (cast `/Game/Blueprints/UI/3DWeaponCatalog/WBP_WeaponInformationPanel` (`WidgetComponent.GetUserWidgetObject` _output)))
        (`/Game/Blueprints/UI/3DWeaponCatalog/WBP_WeaponInformationPanel.Set Fields` _aswbp_weapon_information_panel (break `/Game/Blueprints/Weapons/InteractableWeaponData/FWeaponHotSpotTableRowBase` _array_element) (`.Description_7_2D113C634C52A5D145BFB18EA9A5AB07` (break `/Game/Blueprints/Weapons/InteractableWeaponData/FWeaponHotSpotTableRowBase` _array_element)) (`.Image_11_471523984CB09A648628F1AB1B9E3F8C` (break `/Game/Blueprints/Weapons/InteractableWeaponData/FWeaponHotSpotTableRowBase` _array_element)))))))

(fn `SetPanelRefs`
  (bind _aswbp_info_panel_button (cast `/Game/Blueprints/UI/3DWeaponCatalog/WBP_InfoPanelButton` (`WidgetComponent.GetUserWidgetObject` (`self.WeaponHotspot`))))
  (bind _aswbp_weapon_information_panel (cast `/Game/Blueprints/UI/3DWeaponCatalog/WBP_WeaponInformationPanel` (`WidgetComponent.GetUserWidgetObject` (`self.WeaponInfoPanel`))))
  (set `/Game/Blueprints/UI/3DWeaponCatalog/WBP_InfoPanelButton.InfoPanelRef` _aswbp_weapon_information_panel _aswbp_info_panel_button)
  (bind _aswbp_info_panel_button_2 (cast `/Game/Blueprints/UI/3DWeaponCatalog/WBP_InfoPanelButton` (`WidgetComponent.GetUserWidgetObject` (`self.AmmoHotspot`))))
  (bind _aswbp_weapon_information_panel_2 (cast `/Game/Blueprints/UI/3DWeaponCatalog/WBP_WeaponInformationPanel` (`WidgetComponent.GetUserWidgetObject` (`self.AmmoInfoPanel`))))
  (set `/Game/Blueprints/UI/3DWeaponCatalog/WBP_InfoPanelButton.InfoPanelRef` _aswbp_weapon_information_panel_2 _aswbp_info_panel_button_2)
  (bind _aswbp_info_panel_button_3 (cast `/Game/Blueprints/UI/3DWeaponCatalog/WBP_InfoPanelButton` (`WidgetComponent.GetUserWidgetObject` (`self.MagazineHotspot`))))
  (bind _aswbp_weapon_information_panel_3 (cast `/Game/Blueprints/UI/3DWeaponCatalog/WBP_WeaponInformationPanel` (`WidgetComponent.GetUserWidgetObject` (`self.MagazineInfoPanel`))))
  (set `/Game/Blueprints/UI/3DWeaponCatalog/WBP_InfoPanelButton.InfoPanelRef` _aswbp_weapon_information_panel_3 _aswbp_info_panel_button_3))

(fn `UnequipAttachment`
  (params (attachmentType :type "/Game/Blueprints/Weapons/EAttachmentType Enum" :default "NewEnumerator0")))

(fn `UpdateAttachmentMap`)

(fn `UserConstructionScript`
  (`parent.UserConstructionScript`))